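; Elevator Blueprint that moves a Platform component between two placed marker transforms, Top and Bottom.
; BeginPlay caches both markers' world transforms, destroys the markers and applies Rate as the timeline play rate.
; ElevatorTimeline's update lerps the cached transforms by its Alpha track and teleports the platform without sweeping.
; No node in the graph starts the timeline.
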(event `self.ReceiveBeginPlay`
  (set `self.Top Transform` (`SceneComponent.K2_GetComponentToWorld` (`self.Top`)))
  (set `self.Bottom Transform` (`SceneComponent.K2_GetComponentToWorld` (`self.Bottom`)))
  (`ActorComponent.K2_DestroyComponent` (`self.Top`))
  (`ActorComponent.K2_DestroyComponent` (`self.Bottom`))
  (`TimelineComponent.SetPlayRate` (`self.Elevator Timeline`) (`self.Rate`)))

(fn `UserConstructionScript`)