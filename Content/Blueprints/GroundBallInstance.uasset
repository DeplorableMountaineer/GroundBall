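; GroundBallInstance is the game instance that runs the front-end state machine, from splash screen through title, main menu, new game, load and settings screens.
; Init enters the splash state after a short delay, then advances to Title on a timer.
; Transition removes the old state's widget, records state and entry time, creates the new widget and notifies the game state.
; GroundBallGameState handles state ticking and other events.
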(event `self.ReceiveInit`
  (`KismetSystemLibrary.Delay` 0.2)
  (`self.Transition` "NewEnumerator0"))

(event `On Enter State`
  (params (`From State` :type "/Game/Blueprints/EGameState Enum" :default "NewEnumerator0"))
  (bind _returnvalue (`GameplayStatics.GetPlayerController` 0))
  (set `self.From State` `From State`)
  (switch `/Game/Blueprints/EGameState` (`self.Current State`)
    (:`NewEnumerator0`
      (bind _returnvalue_2 (`|CreateWidget` "/Game/UI/WBP_Splash.WBP_Splash_C" _returnvalue))
      (bind _output_get (set `self.Current Widget` _returnvalue_2))
      (`UserWidget.AddToViewport` _output_get 0)
      (`KismetSystemLibrary.Delay` (`self.Splash Screen Time`))
      (`self.Transition` "NewEnumerator1"))
    (:`NewEnumerator1`
      (bind _returnvalue_3 (`|CreateWidget` "/Game/UI/WBP_Title.WBP_Title_C" _returnvalue))
      (bind _output_get_2 (set `self.Current Widget` _returnvalue_3))
      (`UserWidget.AddToViewport` _output_get_2 0))
    (:`NewEnumerator2`
      (bind _returnvalue_4 (`|CreateWidget` "/Game/UI/WBP_MainMenu.WBP_MainMenu_C" _returnvalue))
      (bind _output_get_3 (set `self.Current Widget` _returnvalue_4))
      (`UserWidget.AddToViewport` _output_get_3 0))
    (:`NewEnumerator3`
      (bind _returnvalue_5 (`|CreateWidget` "/Game/UI/WBP_StartNewGame.WBP_StartNewGame_C" _returnvalue))
      (bind _output_get_4 (set `self.Current Widget` _returnvalue_5))
      (`UserWidget.AddToViewport` _output_get_4 0))
    (:`NewEnumerator4`
      (bind _returnvalue_6 (`|CreateWidget` "/Game/UI/WBP_LoadGame.WBP_LoadGame_C" _returnvalue))
      (bind _output_get_5 (set `self.Current Widget` _returnvalue_6))
      (`UserWidget.AddToViewport` _output_get_5 0))
    (:`NewEnumerator5`
      (bind _returnvalue_7 (`|CreateWidget` "/Game/UI/WBP_AudioSettings.WBP_AudioSettings_C" _returnvalue))
      (bind _output_get_6 (set `self.Current Widget` _returnvalue_7))
      (`UserWidget.AddToViewport` _output_get_6 0))
    (:`NewEnumerator6`
      (bind _returnvalue_8 (`|CreateWidget` "/Game/UI/WBP_VideoSettings.WBP_VideoSettings_C" _returnvalue))
      (bind _output_get_7 (set `self.Current Widget` _returnvalue_8))
      (`UserWidget.AddToViewport` _output_get_7 0))
    (:`NewEnumerator7`
      (bind _returnvalue_9 (`|CreateWidget` "/Game/UI/WBP_ControlSettings.WBP_ControlSettings_C" _returnvalue))
      (bind _output_get_8 (set `self.Current Widget` _returnvalue_9))
      (`UserWidget.AddToViewport` _output_get_8 0))))

(event `On Exit State`
  (params (`To State` :type "/Game/Blueprints/EGameState Enum" :default "NewEnumerator0"))
  (set `self.To State` `To State`)
  (switch `/Game/Blueprints/EGameState` (`self.Current State`)
    (:`NewEnumerator0`
      _)
    (:`NewEnumerator1`
      _)
    (:`NewEnumerator2`
      _)
    (:`NewEnumerator3`
      _)
    (:`NewEnumerator4`
      _)
    (:`NewEnumerator5`
      _)
    (:`NewEnumerator6`
      _)
    (:`NewEnumerator7`
      _))
  (`Widget.RemoveFromParent` (`self.Current Widget`)))

(fn `Transition`
  (params (`To State` :type "/Game/Blueprints/EGameState Enum" :default "NewEnumerator0"))
  (locals (`Previous State` :type "/Game/Blueprints/EGameState Enum"))
  (`self.On Exit State` `To State`)
  (bind _output_get (set `local.Previous State` (`self.Current State`)))
  (bind _output_get_2 (set `self.Current State` `To State`))
  (set `self.State Entry Time` (`KismetSystemLibrary.GetGameTimeInSeconds`))
  (`self.On Enter State` _output_get)
  (message `/Game/Blueprints/BPI_GameState.Update Game State` (`GameplayStatics.GetGameState`) _output_get_2)
  (`KismetSystemLibrary.PrintString` (`|GetEnumeratorNameAsString` _output_get_2)))