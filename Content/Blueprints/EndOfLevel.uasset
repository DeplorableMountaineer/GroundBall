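; EndOfLevel is a level-finish trigger actor for the physics ball.
; When the ball overlaps it, a retriggerable three-second delay starts, then it checks that the game state message has a specific value and the ball is still inside the Box.
; If so, it transitions the game state message, zeroes the ball's velocities, detaches its controller and stops physics simulation.
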(event `self.ReceiveActorBeginOverlap`
  (params (OtherActor :type "Actor Object Reference"))
  (bind _returnvalue (`GameplayStatics.GetGameState`))
  (bind _asphysics_ball_bp_modified (cast `/Game/RollingBP/Blueprints/PhysicsBallBP_Modified` OtherActor))
  (`KismetSystemLibrary.RetriggerableDelay` 3.0)
  (bind _result (message `/Game/Blueprints/BPI_GameState.Get Game State` _returnvalue))
  (if (and (`|EnumEquality` _result "NewEnumerator10") (`KismetArrayLibrary.Array_Contains` (`PrimitiveComponent.GetOverlappingActors` (`self.Box`) "/Game/RollingBP/Blueprints/PhysicsBallBP_Modified.PhysicsBallBP_Modified_C") _asphysics_ball_bp_modified))
    (message `/Game/Blueprints/BPI_GameState.Transition` _returnvalue "NewEnumerator12")
    (bind _ball (`/Game/RollingBP/Blueprints/PhysicsBallBP_Modified.Ball` _asphysics_ball_bp_modified))
    (`PrimitiveComponent.SetAllPhysicsAngularVelocityInDegrees` _ball (0.0 0.0 0.0) false)
    (`PrimitiveComponent.SetAllPhysicsLinearVelocity` _ball (0.0 0.0 0.0) false)
    (`Pawn.DetachFromControllerPendingDestroy` _asphysics_ball_bp_modified)
    (`PrimitiveComponent.SetSimulatePhysics` _ball false)))

(fn `UserConstructionScript`)