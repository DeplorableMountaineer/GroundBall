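; BP_Wave is an actor that acts as a travelling wave which rises, moves and sinks away.
; It starts almost flat on BeginPlay and, every Tick, offsets its Wave component along local X by Speed.
; Elapsed time drives three phases: Z scale grows over RampUp, holds through Travel, then shrinks over RampDown before the actor destroys itself.
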(event `self.ReceiveBeginPlay`
  (`SceneComponent.SetWorldScale3D` (`self.Wave`) (1.0 1.0 0.01)))

(event `self.ReceiveTick`
  (params (DeltaSeconds :type "Float (single-precision)"))
  (bind _ramp_up (`self.Ramp Up`))
  (bind _ramp_down (`self.Ramp Down`))
  (bind _returnvalue (+ _ramp_up (`self.Travel`)))
  (`SceneComponent.K2_AddLocalOffset` (`self.Wave`) (`KismetMathLibrary.MakeVector` (* DeltaSeconds (`self.Speed`))) false false)
  (bind _output_get (set `self.Total Time` (+ (`self.Total Time`) DeltaSeconds)))
  (if (<= _output_get _ramp_up)
    (`SceneComponent.SetWorldScale3D` (`self.Wave`) (`KismetMathLibrary.MakeVector` 1.0 1.0 (/ _output_get _ramp_up)))
    (elif (not (<= _output_get _returnvalue))
      (`SceneComponent.SetWorldScale3D` (`self.Wave`) (`KismetMathLibrary.MakeVector` 1.0 1.0 (- 1.0 (/ (- _output_get _returnvalue) _ramp_down))))
      (if (>= _output_get (+ _returnvalue _ramp_down))
        (`self.K2_DestroyActor`)))))

(fn `UserConstructionScript`)