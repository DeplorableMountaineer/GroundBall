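; GameInstance for the GroundBall game that runs the overall flow from splash and menus through levels, respawns and end of game.
; A state machine: Transition fires exit and enter handlers that swap widgets, open levels in sequence and respawn the ball at a recorded spawn point.
; GroundBallGameState ticks it and receives each state change.
; Progress and audio volumes load on Init and save after levels and audio settings.
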(event `self.ReceiveInit`
  (bind _returnvalue (`GameplayStatics.LoadGameFromSlot` "groundball"))
  (bind _assaved_state (cast `/Game/Blueprints/SavedState` _returnvalue)
    (:`then`
      (set `self.Max Level` (`/Game/Blueprints/SavedState.Level Achieved` _assaved_state))
      (set `self.SFX Volume` (`/Game/Blueprints/SavedState.SFX Volume` _assaved_state))
      (set `self.Music Volume` (`/Game/Blueprints/SavedState.Music Volume` _assaved_state)))
    (:`CastFailed`
      _))
  (`KismetSystemLibrary.Delay` 0.2)
  (`self.Transition` "NewEnumerator0"))

(event `On Enter State`
  (params (`From State` :type "/Game/Blueprints/EGameState Enum" :default "NewEnumerator0"))
  (bind _returnvalue (`GameplayStatics.GetPlayerController` 0))
  (bind _current_level (`self.Current Level`))
  (set `self.From State` `From State`)
  (switch `/Game/Blueprints/EGameState` (`self.Current State`)
    (:`NewEnumerator0`
      (bind _returnvalue_2 (`|CreateWidget` "/Game/UI/WBP_Splash.WBP_Splash_C" _returnvalue))
      (bind _output_get (set `self.Current Widget` _returnvalue_2))
      (`UserWidget.AddToViewport` _output_get 0)
      (`KismetSystemLibrary.Delay` (`self.Splash Screen Time`))
      (`self.Transition` "NewEnumerator1"))
    (:`NewEnumerator1`
      (bind _returnvalue_3 (`|CreateWidget` "/Game/UI/WBP_Title.WBP_Title_C" _returnvalue))
      (bind _output_get_2 (set `self.Current Widget` _returnvalue_3))
      (`UserWidget.AddToViewport` _output_get_2 0))
    (:`NewEnumerator2`
      (bind _returnvalue_4 (`|CreateWidget` "/Game/UI/WBP_MainMenu.WBP_MainMenu_C" _returnvalue))
      (bind _output_get_3 (set `self.Current Widget` _returnvalue_4))
      (`UserWidget.AddToViewport` _output_get_3 0))
    (:`NewEnumerator3`
      (`GameplayStatics.OpenLevel` (`|GetArrayItem` (`self.Level Sequence`) (`self.Current Level`)))
      (`KismetSystemLibrary.Delay` 0.2)
      (`self.Transition` "NewEnumerator9"))
    (:`NewEnumerator4`
      (bind _returnvalue_5 (`|CreateWidget` "/Game/UI/WBP_LoadGame.WBP_LoadGame_C" _returnvalue))
      (bind _output_get_4 (set `self.Current Widget` _returnvalue_5))
      (`UserWidget.AddToViewport` _output_get_4 0))
    (:`NewEnumerator5`
      (bind _returnvalue_6 (`|CreateWidget` "/Game/UI/WBP_AudioSettings.WBP_AudioSettings_C" _returnvalue))
      (bind _output_get_5 (set `self.Current Widget` _returnvalue_6))
      (`UserWidget.AddToViewport` _output_get_5 0))
    (:`NewEnumerator6`
      (bind _returnvalue_7 (`|CreateWidget` "/Game/UI/WBP_VideoSettings.WBP_VideoSettings_C" _returnvalue))
      (bind _output_get_6 (set `self.Current Widget` _returnvalue_7))
      (`UserWidget.AddToViewport` _output_get_6 0))
    (:`NewEnumerator7`
      (bind _returnvalue_8 (`|CreateWidget` "/Game/UI/WBP_ControlSettings.WBP_ControlSettings_C" _returnvalue))
      (bind _output_get_7 (set `self.Current Widget` _returnvalue_8))
      (`UserWidget.AddToViewport` _output_get_7 0))
    (:`NewEnumerator9`
      (bind _returnvalue_9 (`|CreateWidget` "/Game/UI/WBP_LevelTitle.WBP_LevelTitle_C" _returnvalue))
      (`TextBlock.SetText` (`/Game/UI/WBP_LevelTitle.LevelTitle` _returnvalue_9) (`|GetArrayItem` (`self.Level Sequence Friendly Names`) _current_level))
      (`Widget.SetVisibility` (`/Game/UI/WBP_LevelTitle.ProgressSaved` _returnvalue_9) (select `int` _current_level :`0` "Hidden" :`1` "Visible" :`2` "Visible" :`3` "Visible" :`4` "Visible" :`5` "Visible" :`6` "Visible" :`7` "Visible" :`8` "Visible" :`9` "Visible" :`10` "Visible" :!type "ESlateVisibility Enum"))
      (bind _output_get_8 (set `self.Current Widget` _returnvalue_9))
      (`UserWidget.AddToViewport` _output_get_8 0)
      (`KismetSystemLibrary.Delay` 3.0)
      (`self.Transition` "NewEnumerator10")
      (bind _returnvalue_10 (`GameplayStatics.GetActorOfClass` "/Game/RollingBP/Blueprints/PhysicsBallBP_Modified.PhysicsBallBP_Modified_C"))
      (`/Engine/EditorBlueprintResources/StandardMacros.IsValid` _returnvalue_10
        (:`Is Valid`
          (set `self.Spawn Point` (`Actor.K2_GetActorLocation` _returnvalue_10)))
        (:`Is Not Valid`
          (bind _returnvalue_11 (`GameplayStatics.GetActorOfClass` "/Script/Engine.PlayerStart"))
          (`/Engine/EditorBlueprintResources/StandardMacros.IsValid` _returnvalue_11
            (:`Is Valid`
              (set `self.Spawn Point` (`Actor.K2_GetActorLocation` _returnvalue_11)))))))
    (:`NewEnumerator11`
      (`KismetSystemLibrary.Delay` 0.2)
      (bind _returnvalue_12 (`|SpawnActorFromClass` "/Game/RollingBP/Blueprints/PhysicsBallBP_Modified.PhysicsBallBP_Modified_C" (`KismetMathLibrary.MakeTransform` (`self.Spawn Point`)) "AlwaysSpawn" "OverrideRootScale" null null))
      (`Controller.Possess` (`GameplayStatics.GetPlayerController` 0) _returnvalue_12)
      (`KismetSystemLibrary.Delay` 0.2)
      (`self.Transition` "NewEnumerator10"))
    (:`NewEnumerator12`
      (bind _result (`/Engine/EditorBlueprintResources/StandardMacros.IncrementInt` (`self.Current Level`))
        (:`  `
          (`self.Save State`)
          (if (>= _result (`KismetArrayLibrary.Array_Length` (`self.Level Sequence`)))
            (`KismetSystemLibrary.Delay` 0.2)
            (`self.Transition` "NewEnumerator13")
            (else
              (`GameplayStatics.OpenLevel` (`|GetArrayItem` (`self.Level Sequence`) (`self.Current Level`)))
              (`KismetSystemLibrary.Delay` 0.2)
              (`self.Transition` "NewEnumerator9"))))))
    (:`NewEnumerator13`
      (`KismetSystemLibrary.Delay` 0.2)
      (`self.Transition` "NewEnumerator1"))))

(event `On Exit State`
  (params (`To State` :type "/Game/Blueprints/EGameState Enum" :default "NewEnumerator0"))
  (set `self.To State` `To State`)
  (switch `/Game/Blueprints/EGameState` (`self.Current State`)
    (:`NewEnumerator0`
      _)
    (:`NewEnumerator1`
      _)
    (:`NewEnumerator2`
      _)
    (:`NewEnumerator4`
      _)
    (:`NewEnumerator5`
      (`self.Save State`))
    (:`NewEnumerator6`
      _)
    (:`NewEnumerator7`
      _)
    (:`NewEnumerator9`
      _))
  (`Widget.RemoveFromParent` (`self.Current Widget`)))

(fn `Save State`
  (bind _returnvalue (`GameplayStatics.CreateSaveGameObject` "/Game/Blueprints/SavedState.SavedState_C"))
  (set `/Game/Blueprints/SavedState.SFX Volume` (`self.SFX Volume`) _returnvalue)
  (set `/Game/Blueprints/SavedState.Music Volume` (`self.Music Volume`) _returnvalue)
  (bind _output_get (set `self.Max Level` (`KismetMathLibrary.Max` (`self.Current Level`) (`self.Max Level`))))
  (set `/Game/Blueprints/SavedState.Level Achieved` _output_get _returnvalue)
  (`GameplayStatics.SaveGameToSlot` _returnvalue "groundball"))

(fn `Transition`
  (params (`To State` :type "/Game/Blueprints/EGameState Enum" :default "NewEnumerator0"))
  (locals (`Previous State` :type "/Game/Blueprints/EGameState Enum"))
  (`self.On Exit State` `To State`)
  (bind _output_get (set `local.Previous State` (`self.Current State`)))
  (bind _output_get_2 (set `self.Current State` `To State`))
  (set `self.State Entry Time` (`KismetSystemLibrary.GetGameTimeInSeconds`))
  (`self.On Enter State` _output_get)
  (message `/Game/Blueprints/BPI_GameState.Update Game State` (`GameplayStatics.GetGameState`) _output_get_2)
  (`KismetSystemLibrary.PrintString` (`|GetEnumeratorNameAsString` _output_get_2)))