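; BP_WaveMaker is a placeable spawner that periodically emits moving wave actors.
; It sets its tick interval to SpawnInterval, so each Tick spawns one WaveActor at the rear edge of the RampUp box, using the root's rotation.
; The RampUp, Wave and RampDown box lengths are divided by Speed to give each wave its ramp-up, travel and ramp-down durations.
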(event `self.ReceiveBeginPlay`
  (`self.SetActorTickInterval` (`self.Spawn Interval`)))

(event `self.ReceiveTick`
  (params (DeltaSeconds :type "Float (single-precision)"))
  (bind _ramp_up (`self.Ramp Up`))
  (bind _speed (`self.Speed`))
  (bind _boxextent (`BoxComponent.BoxExtent` _ramp_up))
  (`|SpawnActorFromClass` (`self.Wave Actor`) (`KismetMathLibrary.MakeTransform` (- (`SceneComponent.K2_GetComponentLocation` _ramp_up) (* _boxextent (`self.GetActorForwardVector`))) (`SceneComponent.K2_GetComponentRotation` (`self.DefaultSceneRoot`))) "AlwaysSpawn" "OverrideRootScale" null _speed (* (/ (.x _boxextent) _speed) 2.0) (* (/ (.x (`BoxComponent.BoxExtent` (`self.Ramp Down`))) _speed) 2.0) (* (/ (.x (`BoxComponent.BoxExtent` (`self.Wave`))) _speed) 2.0) null))

(fn `UserConstructionScript`)