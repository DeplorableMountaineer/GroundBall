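; GroundBallGameState holds the current game state for the Ground Ball game and exposes it through a getter.
; UpdateGameState stores a new state, while Transition forwards the requested state to GroundBallInstance, the game instance, without changing the stored value itself.
; Tick switches on the current state, but no branch has any logic attached.
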(event `/Game/Blueprints/BPI_GameState.Update Game State`
  (params (`Current State` :type "/Game/Blueprints/EGameState Enum" :default "NewEnumerator16"))
  (set `self.Current State` `Current State`))

(event `self.ReceiveTick`
  (params (DeltaSeconds :type "Float (single-precision)"))
  (switch `/Game/Blueprints/EGameState` (`self.Current State`)))

(event `/Game/Blueprints/BPI_GameState.Transition`
  (params (`To State` :type "/Game/Blueprints/EGameState Enum" :default "NewEnumerator16"))
  (bind _asground_ball_instance (cast `/Game/Blueprints/GroundBallInstance` (`GameplayStatics.GetGameInstance`)))
  (`/Game/Blueprints/GroundBallInstance.Transition` _asground_ball_instance `To State`))

(fn `Get Game State`
  (returns (Result :type "/Game/Blueprints/EGameState Enum"))
  (return (`self.Current State`)))

(fn `UserConstructionScript`)